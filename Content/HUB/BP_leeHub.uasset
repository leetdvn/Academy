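; Hub Blueprint that tracks the state of three minigame widgets (Three Lines, Four Box, Alpha Bet) to maintain an IsKidAFK flag, labeled as tutorial tracking.
; Every Tick switches on Gametype and casts the current widget to the matching game class.
; The flag is true only while that game is running with its GameHistories closed, and stays unchanged if the cast fails.
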(event EventBeginPlay)

(event Collision|EventActorBeginOverlap
  (params (OtherActor :type Actor%20Object%20Reference)))

(event EventTick
  (params (DeltaSeconds :type Float%20%28single-precision%29))
  ;[1 1 1] Tutorial Tracking
  (switch Utilities|FlowControl|Switch|SwitchonlGameType (Variables|Default|Getgametype)
    (:Threelines
      (bind _asthree_line (Utilities|Casting|CastToThreeLine (Variables|Default|GetlCurrentWidget)))
      (if (Variables|/Script/Academy.leeGameHistories|GetisOpened (Variables|/Script/Academy.leeBaseLessions|GetGameHistories _asthree_line))
        (Variables|Default|SetisKidAFK false)
        (elif (Variables|/Script/Academy.leeBaseLessions|GetisGameRuning _asthree_line)
          (Variables|Default|SetisKidAFK true)
          (else
            (Variables|Default|SetisKidAFK false)))))
    (:FourBox
      (bind _asfour_box (Utilities|Casting|CastToFourBox (Variables|Default|GetlCurrentWidget)))
      (if (Variables|/Script/Academy.leeGameHistories|GetisOpened (Variables|/Script/Academy.leeFourBox|GetGameHistories _asfour_box))
        (Variables|Default|SetisKidAFK false)
        (elif (Variables|/Script/Academy.leeFourBox|GetisGameRuning _asfour_box)
          (Variables|Default|SetisKidAFK true)
          (else
            (Variables|Default|SetisKidAFK false)))))
    (:AlphaBet
      (bind _asalpha_bet (Utilities|Casting|CastToAlphaBet (Variables|Default|GetlCurrentWidget)))
      (if (Variables|/Script/Academy.leeGameHistories|GetisOpened (Variables|/Script/Academy.leeAlphaBet|GetGameHistories _asalpha_bet))
        (Variables|Default|SetisKidAFK false)
        (elif (Variables|/Script/Academy.leeAlphaBet|GetisGameRuning _asalpha_bet)
          (Variables|Default|SetisKidAFK true)
          (else
            (Variables|Default|SetisKidAFK false)))))))

(fn ConstructionScript)